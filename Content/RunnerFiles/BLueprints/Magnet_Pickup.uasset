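; Magnet pickup actor for a runner game that temporarily switches on the player's magnet power.
; On overlap with the ThirdPersonCharacter, it sets MagnetActive on that character and hides its mesh.
; After a ten-second delay it clears the flag and destroys itself, with debug prints at both ends.
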(event `self.ReceiveActorBeginOverlap`
  (params (OtherActor :type "Actor Object Reference"))
  (bind _asthird_person_character (cast `/Game/ThirdPersonBP/Blueprints/ThirdPersonCharacter` OtherActor))
  (set `/Game/ThirdPersonBP/Blueprints/ThirdPersonCharacter.MagnetActive` true _asthird_person_character)
  (`KismetSystemLibrary.PrintString` "Magnet Active")
  (`SceneComponent.SetVisibility` (`self.StaticMesh`) false false)
  (`KismetSystemLibrary.Delay` 10.0)
  (cast `/Game/ThirdPersonBP/Blueprints/ThirdPersonCharacter` (`GameplayStatics.GetPlayerCharacter` 0))
  (set `/Game/ThirdPersonBP/Blueprints/ThirdPersonCharacter.MagnetActive` false _asthird_person_character)
  (`KismetSystemLibrary.PrintString` "Magnet Off")
  (`self.K2_DestroyActor`))

(fn `UserConstructionScript`)